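; Teleport point that sends the player's ship to another level, storing a door ID in the game instance.
; On BeginPlay it runs the parent logic and caches the player pawn as BP_Ship.
; When an overlap with Collis ends and Collis still overlaps the ship's collision, it writes TeleportID to DoorID.
; It then opens the level whose name matches the Destination enum value.
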(event OnComponentEndOverlap(Collis)
  (params (OverlappedComponent :type Primitive%20Component%20Object%20Reference) (OtherActor :type Actor%20Object%20Reference) (OtherComp :type Primitive%20Component%20Object%20Reference) (OtherBodyIndex :type Integer))
  ;[1 1 1] Перенести в бонус
  (if (Class|PrimitiveComponent|IsOverlappingComponent (Variables|Default|GetCollis) (Variables|/Script/Arcade.Ship|GetShipCollision (Variables|Default|GetShip)))
    (bind _asbparcade_game_instance (Utilities|Casting|CastToBPArcade_GameInstance (Game|GetGameInstance)))
    (Variables|/Game/BP/BPArcade_GameInstance.BPArcade_GameInstance_C|SetDoorID _asbparcade_game_instance (Variables|Default|GetTeleportID))
    (Game|OpenLevel(byName) (Utilities|String|StringToName (Utilities|String|EnumtoString (Variables|Default|GetDestination))))))

(event EventBeginPlay
  ;[1 1 1] Referens Ship
  (|CallParentFunction)
  (bind _asbp_ship (Utilities|Casting|CastToBP_Ship (Game|Player|GetPlayerPawn 0)))
  (Variables|Default|SetShip _asbp_ship))

(fn ConstructionScript)