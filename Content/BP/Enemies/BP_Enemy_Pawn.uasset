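; BP_Enemy_Pawn is an enemy pawn that chases the player's pawn and shoots.
; On BeginPlay it caches player pawn 0 as Ship and starts its ShootComponent firing.
; Each Tick it moves forward by a fixed local offset, unswept and not scaled by delta time.
; While Ship is valid, it yaws toward it, with the turn clamped by RotatMaxSpeed and scaled by delta seconds.
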(event EventBeginPlay
  (|CallParentFunction)
  (Variables|Default|SetShip (Game|Player|GetPlayerPawn 0))
  (Class|ShootComponent|StartShotting (Variables|Default|GetShootComponent)))

(event EventTick
  (params (DeltaSeconds :type Float%20%28single-precision%29))
  (bind _rotatmaxspeed (Variables|Default|GetRotatMaxSpeed))
  (|CallParentFunction DeltaSeconds)
  (Transformation|AddActorLocalOffset "2.500000, 0, 0" false false)
  (Variables|Default|GetShip
    (:then
      (Transformation|AddActorLocalRotation (Math|Rotator|MakeRotator 0.0 0.0 (* (Math|Float|Clamp(Float) (.yaw (Math|Rotator|Delta(Rotator) (Math|Rotator|FindLookatRotation (Transformation|GetActorLocation) (Transformation|GetActorLocation (Variables|Default|GetShip))) (Transformation|GetActorRotation))) (* -1.0 _rotatmaxspeed) _rotatmaxspeed) (Utilities|Time|GetWorldDeltaSeconds))) false false))
    (:else)))

(fn ConstructionScript)