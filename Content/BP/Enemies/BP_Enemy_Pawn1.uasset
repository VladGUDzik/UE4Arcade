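; BP_Enemy_Pawn1 is an enemy that homes in on the player's pawn, cached as Ship on BeginPlay.
; Each tick it moves forward along its local X axis by a fixed, frame-rate-dependent step, without sweeping for collisions.
; While Ship is valid, it smoothly turns toward it using FindLookAtRotation and RInterpTo, producing a curved pursuit.
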(event EventBeginPlay
  (|CallParentFunction)
  (Variables|Default|SetShip (Game|Player|GetPlayerPawn 0)))

(event EventTick
  (params (DeltaSeconds :type Float%20%28single-precision%29))
  (|CallParentFunction DeltaSeconds)
  (Transformation|AddActorLocalOffset "4.500000, 0, 0" false false)
  (Variables|Default|GetShip
    (:then
      (Transformation|SetActorRotation (Math|Interpolation|RInterpTo (Transformation|GetActorRotation) (Math|Rotator|FindLookatRotation (Transformation|GetActorLocation) (Transformation|GetActorLocation (Variables|Default|GetShip))) (Utilities|Time|GetWorldDeltaSeconds) 2.0)))
    (:else)))

(fn ConstructionScript)