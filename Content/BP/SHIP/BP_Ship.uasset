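; Player ship Blueprint that plays a spinning intro and provides a dash ability with a cooldown.
; On BeginPlay it caps frame rate, then a timeline rolls the mesh and enables movement when finished.
; Dash input runs a timeline that raises speed, disables damage and briefly swaps in a dynamic material fed the reversed forward vector.
; A timer restores dash availability and damageability with sound feedback, and GetDash exposes readiness.
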(event Custom|Dash%20Time
  ;[1 1 1] Dash
  (Variables|Default|SetCanDash true)
  (Variables|Default|SetbCanBeDamaged true)
  (Audio|PlaySound2D "/Game/Assets/Audio/CompileSuccess.CompileSuccess" 1.0 1.0 0.0 0 0))

(event EventBeginPlay
  ;[1 1 1] Rotat Start
  (Development|ExecuteConsoleCommand "t.maxfps 60" 0)
  (Timeline|Spine Play
    (:Update
      (Transformation|AddLocalRotation (Variables|Default|GetShipMesh) (* (Math|Rotator|MakeRotator (+ (Variables|Default|GetYaw) 725.0) 0.0 0.0) (Utilities|Time|GetWorldDeltaSeconds)) false false))
    (:Finished
      (Variables|Default|SetMoveEnab true))))

(event Input|ActionEvents|InputActionDash
  (params (Key :type Key%20Structure :default "None"))
  ;[1 1 1] Dash
  (:Pressed
    (if (Variables|Default|GetCanDash)
      (Audio|PlaySound2D "/Game/Assets/Audio/Bonus/Teleport_Mode_Entered.Teleport_Mode_Entered" 2.0 1.0 0.0 0 0)
      (Timeline|Dash PlayFromStart
        (:Update
          (Variables|Default|SetMoveSpeed (Variables|Default|GetDashSpeed))
          (Variables|Default|SetCanDash false)
          (Variables|Default|SetbCanBeDamaged false)
          (bind _returnvalue (Rendering|Material|CreateDynamicMaterialInstance (Variables|Default|GetShipMesh) 0 "/Game/BP/SHIP/M_Dash_Inst.M_Dash_Inst" "None" :!class /Script/Engine.PrimitiveComponent))
          (bind _output_get (Variables|Default|SetReffeerns _returnvalue))
          (Rendering|Material|SetVectorParameterValue _output_get "Loc" (Math|Conversions|ToLinearColor(Vector) (* (Math|Vector|GetForwardVector (Variables|Default|GetShipCollision)) -1.0)) :!class /Script/Engine.MaterialInstanceDynamic)
          (Utilities|FlowControl|Delay 0.2)
          (Rendering|Material|SetMaterial (Variables|Default|GetShipMesh) 0 "/Game/Material/Meshes/SimplePivotPainterExampleMat.SimplePivotPainterExampleMat")
          (Utilities|Time|SetTimerbyEvent (delegate Custom|Dash%20Time) 2.5))
        (:Finished
          (Variables|Default|SetMoveSpeed 1e+03)))
      (else
        (Audio|PlaySound2D "/Game/Assets/Audio/CompileFailed.CompileFailed" 1.0 1.0 0.0 0 0)))))

(fn ConstructionScript)

(fn GetDash
  (return (Variables|Default|GetCanDash)))