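; Canvas-drawn HUD for an arcade ship game, showing life icons, the score, a pause button and a dash icon tinted dark when GetDash is false.
; DrawHUD redraws each element from game mode, game instance and ship state, using helpers that scale and anchor coordinates to the viewport.
; The pause hit box opens the pause menu, and the game mode's game-over event opens the game-over widget; both pause the game.
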(event Custom|OnGameOver
  (bind _returnvalue (UserInterface|CreateWidget "/Game/BP/HUD/GameOver/WGame_over.WGame_over_C" (Game|Player|GetOwningPlayerController)))
  (UserInterface|Viewport|AddtoViewport _returnvalue 0)
  (Game|SetGamePaused true))

(event EventHitBoxClick
  (params (BoxName :type Name :default "None"))
  (switch name BoxName
    (:Pause
      (bind _returnvalue (UserInterface|CreateWidget "/Game/BP/HUD/PauseMenu/W_PauseMenu.W_PauseMenu_C" (Game|Player|GetOwningPlayerController)))
      (UserInterface|Viewport|AddtoViewport _returnvalue 0)
      (Game|SetGamePaused true))))

(event EventBeginPlay
  (bind _asarcade_game_mode_base (Utilities|Casting|CastToArcadeGameModeBase (Game|GetGameMode)))
  (EventDispatchers|AssignGameOver _asarcade_game_mode_base (delegate Custom|OnGameOver)))

(event EventDrawHUD
  (params (SizeX :type Integer) (SizeY :type Integer))
  (|DrawLive
    (:Completed
      (CallFunction|DrawPauseButtom)
      (CallFunction|DrawPoints)
      (CallFunction|DrawDash))))

(fn ConstructionScript)

(fn ScaleCoords
  (params (in :type Vector%202D%20Structure))
  (return (* in (Class|WidgetLayoutLibrary|GetViewportScale))))

(fn ApplyCoords
  (params (in :type Vector%202D%20Structure) (A :type Vector%202D%20Structure))
  (return (+ in (* A (Viewport|GetViewportSize)))))

(fn DrawPoints
  (bind _out (CallFunction|ScaleCoords "(X=-50.000000,Y=20.000000)"))
  (bind _out_2 (CallFunction|ApplyCoords _out "(X=0.500000,Y=0.000000)"))
  (HUD|DrawText (Utilities|String|ToString(Integer) (Variables|/Script/Arcade.Arcade_GameInstance|GetGamePoints (.AsArcade%20Game%20Instance (Utilities|Casting|CastToArcade_GameInstance (Game|GetGameInstance))))) "(R=1.000000,G=1.000000,B=1.000000,A=1.000000)" (.x _out_2) (.y _out_2) "/Game/Assets/UI/VRText_RobotoLarge.VRText_RobotoLarge" 0.5 false))

(fn DrawPauseButtom
  (bind _out (CallFunction|ScaleCoords "(X=-84.000000,Y=20.000000)"))
  (bind _out_2 (CallFunction|ScaleCoords "(X=64.000000,Y=64.000000)"))
  (bind _out_3 (CallFunction|ApplyCoords _out "(X=1.000000,Y=0.000000)"))
  (Canvas|DrawTexture "/Game/Assets/UI/pause-button.pause-button" (.x _out_3) (.y _out_3) (.x _out_2) (.y _out_2) 0.0 0.0 1.0 1.0 "(R=1.000000,G=1.000000,B=1.000000,A=1.000000)")
  (Class|HUD|AddHitBox (CallFunction|ApplyCoords (CallFunction|ScaleCoords "(X=-84.000000,Y=20.000000)") "(X=1.000000,Y=0.000000)") (CallFunction|ScaleCoords "(X=64.000000,Y=64.000000)") "Pause" false))

(fn DrawDash
  (bind _out (CallFunction|ScaleCoords "(X=64.000000,Y=64.000000)"))
  (bind _out_2 (CallFunction|ScaleCoords "(X=64.000000,Y=64.000000)"))
  (bind _returnvalue (+ 64.0 1e+01))
  (bind _returnvalue_2 (+ 64.0 1e+01))
  (bind _returnvalue_3 (* 0 _returnvalue))
  (bind _returnvalue_4 (* 0 _returnvalue_2))
  (bind _returnvalue_5 (+ _returnvalue_3 -32.0))
  (bind _returnvalue_6 (+ _returnvalue_4 -32.0))
  (bind _returnvalue_7 (Math|Vector2D|MakeVector2D _returnvalue_5 1e+02))
  (bind _returnvalue_8 (Math|Vector2D|MakeVector2D _returnvalue_6 1e+02))
  (bind _out_3 (CallFunction|ScaleCoords _returnvalue_7))
  (bind _out_4 (CallFunction|ScaleCoords _returnvalue_8))
  (bind _out_5 (CallFunction|ApplyCoords _out_3 "(X=0.100000,Y=0.000000)"))
  (bind _out_6 (CallFunction|ApplyCoords _out_4 "(X=0.100000,Y=0.000000)"))
  (bind _asbp_ship (Utilities|Casting|CastToBP_Ship (Game|Player|GetPlayerPawn 0)))
  (bind _dash (Default|GetDash _asbp_ship))
  (if _dash
    (Canvas|DrawTexture "/Game/Assets/UI/dash.dash" (.x _out_6) (.y _out_6) (.x _out_2) (.y _out_2) 0.0 0.0 1.0 1.0 "(R=1.000000,G=1.000000,B=1.000000,A=1.000000)")
    (else
      (Canvas|DrawTexture "/Game/Assets/UI/dash.dash" (.x _out_5) (.y _out_5) (.x _out) (.y _out) 0.0 0.0 1.0 1.0 "(R=0.000000,G=0.007927,B=0.088542,A=1.000000)" "BLEND_Translucent" 1.0 false 0.0 "(X=0.000000,Y=0.000000)"))))